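; Interactable platform actor that toggles its static mesh between its original height and a grown height.
; BeginPlay caches the mesh's starting relative scale.
; Interact calls MC_RequestInteract, which flips PlatformOn and plays or reverses GrowTimeline.
; The timeline's Grow track lerps only the Z scale toward MaxGrowth, leaving X and Y at their original values.
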(event `self.ReceiveBeginPlay`
  (set `self.OriginalScale` (`SceneComponent.RelativeScale3D` (`self.StaticMesh`))))

(event `/Game/Profesor/Clase14/BPI_Interactable.Interact`
  (`self.MC_RequestInteract`))

(event `MC_RequestInteract`
  (bind (_originalscale_x _originalscale_y _originalscale_z) (`KismetMathLibrary.BreakVector` (`self.OriginalScale`)))
  (bind _output_get (set `self.PlatformOn` (not (`self.PlatformOn`))))
  (if _output_get
    (bind (_direction _grow) (`Timeline|GrowTimeline` :!label _label)
      (:`Update`
        (`SceneComponent.SetRelativeScale3D` (`self.StaticMesh`) (`KismetMathLibrary.MakeVector` _originalscale_x _originalscale_y (`KismetMathLibrary.Lerp` _originalscale_z (`self.MaxGrowth`) _grow)))))
    (else
      (goto _label :!via `Reverse`))))

(fn `UserConstructionScript`)