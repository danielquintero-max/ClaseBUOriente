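; BP_TestActor is a test actor with a static mesh whose color can be randomized.
; On BeginPlay it creates a dynamic material instance from M_Cube, stores it and applies it to the mesh.
; MC_ChangeColor, named like a multicast event, sets that instance's CubeColor parameter to a random opaque color.
; The ChangeColor event is empty, and nothing in this Blueprint calls MC_ChangeColor.
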(event `self.ReceiveBeginPlay`
  (bind _returnvalue (`KismetMaterialLibrary.CreateDynamicMaterialInstance` "/Game/Profesor/Clase14/M_Cube.M_Cube"))
  (bind _output_get (set `self.DynamicMat` _returnvalue))
  (`PrimitiveComponent.SetMaterial` (`self.StaticMesh`) 0 _output_get))

(event `ChangeColor`)

(event `MC_ChangeColor`
  (`MaterialInstanceDynamic.SetVectorParameterValue` (`self.DynamicMat`) "CubeColor" (make `LinearColor` (`KismetMathLibrary.RandomFloat`) (`KismetMathLibrary.RandomFloat`) (`KismetMathLibrary.RandomFloat`) 1.0)))

(fn `UserConstructionScript`)