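; PC_MultiplayerTest is a player controller for testing networked interaction in a class exercise.
; BeginPlay sets game-only input, hides the cursor and adds the default Enhanced Input mapping context.
; Server- and multicast-named events forward InteractMessage to an actor, and ServerChangeColor calls an actor's MCChangeColor.
; The cursor-trace logic that would trigger them, including distance and BPI_Interactable checks, is disconnected and never runs.
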(event `self.ReceiveBeginPlay`
  (bind _returnvalue (subsystem `EnhancedInputLocalPlayerSubsystem`))
  (`WidgetBlueprintLibrary.SetInputMode_GameOnly` self)
  (set `self.bShowMouseCursor` false)
  (`/Engine/EditorBlueprintResources/StandardMacros.IsValid` _returnvalue
    (:`Is Valid`
      (`EnhancedInputSubsystemInterface.AddMappingContext` _returnvalue "/Game/FirstPerson/Input/IMC_Default.IMC_Default" 1 (struct)))))

(event `SV_RequestInteract`
  (params (InteractedActor :type "Actor Object Reference"))
  (message `/Game/Profesor/Clase14/BPI_Interactable.Interact` InteractedActor))

(event `MC_RequestInteract`
  (params (InteractedActor :type "Actor Object Reference"))
  (message `/Game/Profesor/Clase14/BPI_Interactable.Interact` InteractedActor))

(event `ServerChangeColor`
  (params (NewParam :type "/Game/Profesor/Clase14/BP_TestActor Object Reference"))
  (`/Game/Profesor/Clase14/BP_TestActor.MC_ChangeColor` NewParam))

(event `Key|LeftMouseButton` :consume false
  (params (Key :type "Key Structure")))

(fn `UserConstructionScript`)