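; Interactable actor that toggles its spotlight on and off.
; BeginPlay caches the spotlight's starting intensity as MaxIntensity.
; Interact hands off to MC_RequestInteract, which flips LightIsOn and sets the intensity to either the cached value or zero.
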(event `self.ReceiveBeginPlay`
  (set `self.MaxIntensity` (`LightComponentBase.Intensity` (`self.SpotLight`))))

(event `/Game/Profesor/Clase14/BPI_Interactable.Interact`
  (`self.MC_RequestInteract`))

(event `MC_RequestInteract`
  (bind _output_get (set `self.LightIsOn` (not (`self.LightIsOn`))))
  (if _output_get
    (`LightComponent.SetIntensity` (`self.SpotLight`) (`self.MaxIntensity`))
    (else
      (`LightComponent.SetIntensity` (`self.SpotLight`) 0.0))))

(fn `UserConstructionScript`)