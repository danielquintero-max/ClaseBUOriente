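; BP_InteractionCube is a networked cube that changes to a random color when a third-person character enters its sphere trigger.
; On BeginPlay it creates a dynamic instance of M_Cube and applies it to the static mesh.
; Only the authority rolls the new color on overlap, storing it in the RepNotify variable NewCubeColor, whose OnRep updates the material's CubeColor parameter.
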(event `self.ReceiveBeginPlay`
  (bind _returnvalue (`KismetMaterialLibrary.CreateDynamicMaterialInstance` "/Game/Profesor/Clase14/M_Cube.M_Cube"))
  (bind _output_get (set `self.CubeMat` _returnvalue))
  (`PrimitiveComponent.SetMaterial` (`self.StaticMesh`) 0 _output_get))

(event `self.Sphere.OnComponentBeginOverlap`
  (params (OverlappedComponent :type "PrimitiveComponent Object Reference") (OtherActor :type "Actor Object Reference") (OtherComp :type "PrimitiveComponent Object Reference") (OtherBodyIndex :type Integer) (bFromSweep :type Boolean) (SweepResult :type "HitResult Structure (by ref)"))
  (`/Engine/EditorBlueprintResources/ActorMacros.Switch Has Authority`
    (:`Authority`
      (cast `/Game/ThirdPerson/Blueprints/BP_ThirdPersonCharacter` OtherActor)
      (set `self.NewCubeColor` (make `LinearColor` (`KismetMathLibrary.RandomFloat`) (`KismetMathLibrary.RandomFloat`) (`KismetMathLibrary.RandomFloat`) 1.0)))))

(fn `OnRep_NewCubeColor`
  (`MaterialInstanceDynamic.SetVectorParameterValue` (`self.CubeMat`) "CubeColor" (`self.NewCubeColor`)))

(fn `UserConstructionScript`)