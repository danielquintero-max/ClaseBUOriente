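; BP_BallPawn is a player-controlled physics ball pawn driven by Enhanced Input.
; Look input rotates the controller, and move input pushes the sphere with forces along the control yaw's forward and right vectors.
; Jump applies an upward impulse scaled by JumpPower, but only when a short downward line trace from the actor finds ground.
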(event `EnhancedInput|/Game/ThirdPerson/Input/Actions/IA_Look`
  (params (ActionValue :type "Vector2D Structure") (ElapsedSeconds :type "Float (double-precision)") (TriggeredSeconds :type "Float (double-precision)") (InputAction :type "InputAction Object Reference" :default "/Game/ThirdPerson/Input/Actions/IA_Look.IA_Look"))
  (bind (_x _y) (`KismetMathLibrary.BreakVector2D` ActionValue))
  (:`Triggered`
    (`self.AddControllerYawInput` _x)
    (`self.AddControllerPitchInput` _y)))

(event `EnhancedInput|/Game/ThirdPerson/Input/Actions/IA_Move`
  (params (ActionValue :type "Vector2D Structure") (ElapsedSeconds :type "Float (double-precision)") (TriggeredSeconds :type "Float (double-precision)") (InputAction :type "InputAction Object Reference" :default "/Game/ThirdPerson/Input/Actions/IA_Move.IA_Move"))
  (bind (_x _y) (`KismetMathLibrary.BreakVector2D` ActionValue))
  (bind _returnvalue (`KismetMathLibrary.MakeRotator` 0.0 0.0 (.yaw (`self.GetControlRotation`))))
  (:`Triggered`
    (`PrimitiveComponent.AddForce` (`self.Sphere`) (* _y (`KismetMathLibrary.GetForwardVector` _returnvalue) 50000.0) "None" false)
    (`PrimitiveComponent.AddForce` (`self.Sphere`) (* _x (`KismetMathLibrary.GetRightVector` _returnvalue) 50000.0) "None" false)))

(event `EnhancedInput|/Game/ThirdPerson/Input/Actions/IA_Jump`
  (params (ActionValue :type Boolean) (ElapsedSeconds :type "Float (double-precision)") (TriggeredSeconds :type "Float (double-precision)") (InputAction :type "InputAction Object Reference" :default "/Game/ThirdPerson/Input/Actions/IA_Jump.IA_Jump"))
  (bind _returnvalue (`self.K2_GetActorLocation`))
  (:`Triggered`
    (bind (_outhit _returnvalue_2) (`KismetSystemLibrary.LineTraceSingle` _returnvalue (- _returnvalue (0.0 0.0 100.0)) "TraceTypeQuery1" false (`|MakeArray` self :!type "Actor Object Reference")))
    (if _returnvalue_2
      (`PrimitiveComponent.AddImpulse` (`self.Sphere`) (`KismetMathLibrary.MakeVector` 0.0 0.0 (`self.JumpPower`)) "None" false))))

(fn `UserConstructionScript`)