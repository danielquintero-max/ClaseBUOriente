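; BPC_Attack is an actor component that gives its owner a forward attack and an area-of-effect attack.
; The forward attack sphere-traces a short distance ahead and damages the BPC_Health component of the first actor hit.
; The AOE attack multi-sphere-traces around the owner, using a temporary hit list so each actor with BPC_Health takes damage only once per attack.
; Both traces ignore the owner and draw debug shapes.
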(event `ForwardAttack`
  (bind _returnvalue (`self.GetOwner`))
  (bind _returnvalue_2 (`Actor.K2_GetActorLocation` _returnvalue))
  (bind (_outhit _returnvalue_3) (`KismetSystemLibrary.SphereTraceSingleForObjects` _returnvalue_2 (+ _returnvalue_2 (* (`Actor.GetActorForwardVector` _returnvalue) 300.0)) 10.0 (`|MakeArray` "ObjectTypeQuery1" "ObjectTypeQuery2" "ObjectTypeQuery3" "ObjectTypeQuery6" :!type "EObjectTypeQuery Enum") false (`|MakeArray` (`self.GetOwner`)) "ForDuration" true (struct :`R` 1.0 :`A` 1.0) (struct :`G` 1.0 :`A` 1.0) 0.5))
  (if _returnvalue_3
    (bind _returnvalue_4 (`Actor.GetComponentByClass` (`.HitActor` (`GameplayStatics.BreakHitResult` _outhit)) "/Game/Profesor/Clase15/Components/BPC_Health.BPC_Health_C"))
    (`/Engine/EditorBlueprintResources/StandardMacros.IsValid` _returnvalue_4
      (:`Is Valid`
        (`/Game/Profesor/Clase15/Components/BPC_Health.TakeDamage` _returnvalue_4 (`self.ForwardAttackDamage`))))))

(event `AOE_Attack`
  (bind _returnvalue (`Actor.K2_GetActorLocation` (`self.GetOwner`)))
  (bind (_outhits _returnvalue_2) (`KismetSystemLibrary.SphereTraceMultiForObjects` _returnvalue _returnvalue (`self.AOE_Radius`) (`|MakeArray` "ObjectTypeQuery1" "ObjectTypeQuery2" "ObjectTypeQuery3" "ObjectTypeQuery6" :!type "EObjectTypeQuery Enum") false (`|MakeArray` (`self.GetOwner`)) "ForDuration" true (struct :`R` 1.0 :`A` 1.0) (struct :`G` 1.0 :`A` 1.0) 0.5))
  (if _returnvalue_2
    (for _array_element _outhits
      (bind (_bblockinghit _binitialoverlap _time _distance _location _impactpoint _normal _impactnormal _physmat _hitactor) (`GameplayStatics.BreakHitResult` _array_element))
      (bind _returnvalue_3 (`Actor.GetComponentByClass` _hitactor "/Game/Profesor/Clase15/Components/BPC_Health.BPC_Health_C"))
      (`/Engine/EditorBlueprintResources/StandardMacros.IsValid` _returnvalue_3
        (:`Is Valid`
          (if (not (`KismetArrayLibrary.Array_Contains` (`self.Hitted Actors`) _hitactor))
            (`KismetArrayLibrary.Array_AddUnique` (`self.Hitted Actors`) _hitactor)
            (`/Game/Profesor/Clase15/Components/BPC_Health.TakeDamage` _returnvalue_3 (`self.AOEDamage`))))))
    (`KismetArrayLibrary.Array_Clear` (`self.Hitted Actors`))))