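; Actor component that gives its owner health and a floating health bar.
; On BeginPlay it adds a screen-space, collision-free WidgetComponent above the owner and fills it with a WBP_HealthBar, passing in Health and the owner.
; TakeDamage subtracts from Health, fires OnDamageTaken, and also fires OnDefeat whenever the result is zero or below, with no clamping.
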(event `self.ReceiveBeginPlay`
  (bind _returnvalue (`|AddComponentByClass` (`self.GetOwner`) "/Script/UMG.WidgetComponent" false (`KismetMathLibrary.MakeTransform` (0.0 0.0 100.0))))
  (set `self.AddedWidget` _returnvalue)
  (`WidgetComponent.SetDrawSize` (`self.AddedWidget`) (150.0 10.0))
  (`WidgetComponent.SetWidgetSpace` (`self.AddedWidget`) "Screen")
  (`PrimitiveComponent.SetCollisionEnabled` (`self.AddedWidget`) "NoCollision")
  (bind _returnvalue_2 (`|CreateWidget` "/Game/Profesor/Clase15/Components/WBP_HealthBar.WBP_HealthBar_C" null (`self.Health`) (`self.GetOwner`)))
  (`WidgetComponent.SetWidget` (`self.AddedWidget`) _returnvalue_2))

(fn `TakeDamage`
  (params (Damage :type "Float (double-precision)"))
  (set `self.Health` (- (`self.Health`) Damage))
  (`self.OnDamageTaken`)
  (if (<= (`self.Health`) 0.0)
    (`self.OnDefeat`)))