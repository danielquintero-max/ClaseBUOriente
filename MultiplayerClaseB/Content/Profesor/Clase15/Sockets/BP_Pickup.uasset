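; BP_Pickup is a pickup actor that can be picked up and dropped, with its mesh chosen per instance.
; The construction script applies the PickupStaticMesh variable to PickupMesh.
; Pickup turns off physics simulation and collision on the mesh, and Drop restores both so it becomes a physical object again.
; Attachment to a holder is not handled in this Blueprint.
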(event `Pickup`
  (bind _pickupmesh (`self.PickupMesh`))
  (`PrimitiveComponent.SetSimulatePhysics` _pickupmesh false)
  (`PrimitiveComponent.SetCollisionEnabled` _pickupmesh "NoCollision"))

(event `Drop`
  (bind _pickupmesh (`self.PickupMesh`))
  (`PrimitiveComponent.SetSimulatePhysics` _pickupmesh true)
  (`PrimitiveComponent.SetCollisionEnabled` _pickupmesh "QueryAndPhysics"))

(fn `UserConstructionScript`
  (`StaticMeshComponent.SetStaticMesh` (`self.PickupMesh`) (`self.PickupStaticMesh`)))