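; Test area actor that changes its own look and the third-person character's shoulder decal while the character is inside its sphere.
; On BeginPlay it creates a dynamic material instance of M_Prueba and applies it to its static mesh.
; Sphere overlap begin and end switch that material's color, scalar and texture parameters between entry and exit values.
; The same events set logo color and intensity on the overlapping character's DecalHombro.
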(event `self.ReceiveBeginPlay`
  (bind _returnvalue (`KismetMaterialLibrary.CreateDynamicMaterialInstance` "/Game/Profesor/Clase10/M_Prueba.M_Prueba"))
  (set `self.ReferenciaMaterial` _returnvalue)
  (`PrimitiveComponent.SetMaterial` (`self.StaticMesh`) 0 (`self.ReferenciaMaterial`)))

(event `self.Sphere.OnComponentBeginOverlap`
  (params (OverlappedComponent :type "PrimitiveComponent Object Reference") (OtherActor :type "Actor Object Reference") (OtherComp :type "PrimitiveComponent Object Reference") (OtherBodyIndex :type Integer) (bFromSweep :type Boolean) (SweepResult :type "HitResult Structure (by ref)"))
  (bind _asbp_third_person_character (cast `/Game/ThirdPerson/Blueprints/BP_ThirdPersonCharacter` OtherActor))
  (`|ExecutionSequence`
    (:`then_0`
      (`MaterialInstanceDynamic.SetVectorParameterValue` (`self.ReferenciaMaterial`) "NombreDeColor" (`self.ColorDeEntrada`))
      (`MaterialInstanceDynamic.SetScalarParameterValue` (`self.ReferenciaMaterial`) "ValorFlotante" 50.0)
      (`MaterialInstanceDynamic.SetTextureParameterValue` (`self.ReferenciaMaterial`) "ParametroTextura" (`self.TexturaEntrada`)))
    (:`then_1`
      (bind _decalhombro (`/Game/ThirdPerson/Blueprints/BP_ThirdPersonCharacter.DecalHombro` _asbp_third_person_character))
      (`MaterialInstanceDynamic.SetVectorParameterValue` _decalhombro "LogoColor" (`self.ColorDeEntrada`))
      (`MaterialInstanceDynamic.SetScalarParameterValue` _decalhombro "LogoIntensity" 50.0))))

(event `self.Sphere.OnComponentEndOverlap`
  (params (OverlappedComponent :type "PrimitiveComponent Object Reference") (OtherActor :type "Actor Object Reference") (OtherComp :type "PrimitiveComponent Object Reference") (OtherBodyIndex :type Integer))
  (bind _asbp_third_person_character (cast `/Game/ThirdPerson/Blueprints/BP_ThirdPersonCharacter` OtherActor))
  (`|ExecutionSequence`
    (:`then_0`
      (`MaterialInstanceDynamic.SetVectorParameterValue` (`self.ReferenciaMaterial`) "NombreDeColor" (`self.ColorDeSalida`))
      (`MaterialInstanceDynamic.SetScalarParameterValue` (`self.ReferenciaMaterial`) "ValorFlotante" 0.0)
      (`MaterialInstanceDynamic.SetTextureParameterValue` (`self.ReferenciaMaterial`) "ParametroTextura" (`self.TexturaSalida`)))
    (:`then_1`
      (bind _decalhombro (`/Game/ThirdPerson/Blueprints/BP_ThirdPersonCharacter.DecalHombro` _asbp_third_person_character))
      (`MaterialInstanceDynamic.SetVectorParameterValue` _decalhombro "LogoColor" (`self.ColorDeSalida`))
      (`MaterialInstanceDynamic.SetScalarParameterValue` _decalhombro "LogoIntensity" 0.0))))

(fn `UserConstructionScript`)