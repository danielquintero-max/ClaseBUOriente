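; BP_Area is a trigger area that recolors itself and the third-person character as the character enters or leaves its sphere.
; On BeginPlay it puts a dynamic instance of M_Ejemplo on its static mesh.
; Sphere overlap events set color parameters on that material and the character's material, turning the character's glow on inside and off outside.
; Unconnected logic for a post-process blendable material with a changing Resolution parameter never runs.
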(event `self.ReceiveBeginPlay`
  (bind _returnvalue (`KismetMaterialLibrary.CreateDynamicMaterialInstance` "/Game/Profesor/Clase10/M_Ejemplo.M_Ejemplo"))
  (set `self.ReferenciaMaterial` _returnvalue)
  (`PrimitiveComponent.SetMaterial` (`self.StaticMesh`) 0 (`self.ReferenciaMaterial`)))

(event `self.Sphere.OnComponentBeginOverlap`
  (params (OverlappedComponent :type "PrimitiveComponent Object Reference") (OtherActor :type "Actor Object Reference") (OtherComp :type "PrimitiveComponent Object Reference") (OtherBodyIndex :type Integer) (bFromSweep :type Boolean) (SweepResult :type "HitResult Structure (by ref)"))
  (bind _asbp_third_person_character (cast `/Game/ThirdPerson/Blueprints/BP_ThirdPersonCharacter` OtherActor))
  (`MaterialInstanceDynamic.SetVectorParameterValue` (`self.ReferenciaMaterial`) "NombreGenericoDeColor" (struct :`R` 0.085961 :`G` 1.0 :`A` 1.0))
  (bind _charactermaterial (`/Game/ThirdPerson/Blueprints/BP_ThirdPersonCharacter.CharacterMaterial` _asbp_third_person_character))
  (`MaterialInstanceDynamic.SetVectorParameterValue` _charactermaterial "ColorTorso" (struct :`R` 1.0 :`G` 0.804122 :`A` 1.0))
  (`MaterialInstanceDynamic.SetScalarParameterValue` _charactermaterial "GlowIntensity" 50.0))

(event `self.Sphere.OnComponentEndOverlap`
  (params (OverlappedComponent :type "PrimitiveComponent Object Reference") (OtherActor :type "Actor Object Reference") (OtherComp :type "PrimitiveComponent Object Reference") (OtherBodyIndex :type Integer))
  (bind _asbp_third_person_character (cast `/Game/ThirdPerson/Blueprints/BP_ThirdPersonCharacter` OtherActor))
  (`MaterialInstanceDynamic.SetVectorParameterValue` (`self.ReferenciaMaterial`) "NombreGenericoDeColor" (struct :`R` 1.0 :`G` 0.042958 :`A` 1.0))
  (bind _charactermaterial (`/Game/ThirdPerson/Blueprints/BP_ThirdPersonCharacter.CharacterMaterial` _asbp_third_person_character))
  (`MaterialInstanceDynamic.SetVectorParameterValue` _charactermaterial "ColorTorso" (struct :`R` 0.087081 :`G` 1.0 :`A` 1.0))
  (`MaterialInstanceDynamic.SetScalarParameterValue` _charactermaterial "GlowIntensity" 0.0))

(fn `UserConstructionScript`)