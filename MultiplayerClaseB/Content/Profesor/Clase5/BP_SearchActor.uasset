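; BP_SearchActor is an actor that cycles the point light color of every BP_InteractionActor in the level.
; On BeginPlay it gathers them with GetAllActorsOfClass and loops over them, setting magenta, blue, then green, with delays between passes.
; A looping timer bound to the RainbowColors event re-enters the same chain to repeat the cycle.
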(event `self.ReceiveBeginPlay`
  (`KismetSystemLibrary.K2_SetTimerDelegate` (delegate `RainbowColors`) 8.0 true)
  (bind _outactors (`GameplayStatics.GetAllActorsOfClass` "/Game/Profesor/Clase5/BP_InteractionActor.BP_InteractionActor_C" :!label _label))
  (for _array_element _outactors
    (`LightComponent.SetLightColor` (`/Game/Profesor/Clase5/BP_InteractionActor.PointLight` _array_element) (struct :`R` 0.92488 :`B` 1.0 :`A` 1.0) true))
  (`KismetSystemLibrary.Delay` 2.0)
  (for _array_element_2 _outactors
    (`LightComponent.SetLightColor` (`/Game/Profesor/Clase5/BP_InteractionActor.PointLight` _array_element_2) (struct :`G` 0.043139 :`B` 1.0 :`A` 1.0) true))
  (`KismetSystemLibrary.Delay` 2.0)
  (for _array_element_3 _outactors
    (`LightComponent.SetLightColor` (`/Game/Profesor/Clase5/BP_InteractionActor.PointLight` _array_element_3) (struct :`G` 1.0 :`B` 0.087788 :`A` 1.0) true)))

(event `RainbowColors`
  (goto _label))

(fn `UserConstructionScript`)