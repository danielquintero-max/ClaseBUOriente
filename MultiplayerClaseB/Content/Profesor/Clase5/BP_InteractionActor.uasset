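; BP_InteractionActor is a proximity light actor, apparently a class exercise, that lights up while the third-person character is nearby.
; Sphere overlap events cast to BP_ThirdPersonCharacter, then switch the PointLight intensity between bright and zero.
; BeginPlay gathers every BP_AnotherActor and loops over them with an empty body.
; Unconnected practice nodes for flow control, actor lookup, light color and mesh swapping never execute.
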(event `self.ReceiveBeginPlay`
  (bind _outactors (`GameplayStatics.GetAllActorsOfClass` "/Game/Profesor/Clase5/BP_AnotherActor.BP_AnotherActor_C"))
  (for _array_element _outactors
    _))

(event `self.Sphere.OnComponentBeginOverlap`
  (params (OverlappedComponent :type "PrimitiveComponent Object Reference") (OtherActor :type "Actor Object Reference") (OtherComp :type "PrimitiveComponent Object Reference") (OtherBodyIndex :type Integer) (bFromSweep :type Boolean) (SweepResult :type "HitResult Structure (by ref)"))
  (cast `/Game/ThirdPerson/Blueprints/BP_ThirdPersonCharacter` OtherActor)
  (`LightComponent.SetIntensity` (`self.PointLight`) 10000.0))

(event `self.Sphere.OnComponentEndOverlap`
  (params (OverlappedComponent :type "PrimitiveComponent Object Reference") (OtherActor :type "Actor Object Reference") (OtherComp :type "PrimitiveComponent Object Reference") (OtherBodyIndex :type Integer))
  (cast `/Game/ThirdPerson/Blueprints/BP_ThirdPersonCharacter` OtherActor)
  (`LightComponent.SetIntensity` (`self.PointLight`) 0.0))

(fn `UserConstructionScript`)