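; Enemy AI Blueprint that turns AI Perception stimuli into Blackboard values on its AI controller.
; Perception updates currently reach only HandleHearing, which stores a heard noise's location as LastKnownLocation and sets Investigating.
; HandleSight would set TargetActor to the seen player, or clear it and save LastKnownLocation when sight is lost, but its call is disconnected from the event.
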(event `self.AIPerception.OnTargetPerceptionUpdated`
  (params (Actor :type "Actor Object Reference") (Stimulus :type "AIStimulus Structure"))
  (`self.HandleHearing` Actor Stimulus))

(fn `HandleHearing`
  (params (SensedActor :type "Actor Object Reference") (Stimulus :type "AIStimulus Structure"))
  (bind ((`StimulusLocation` _stimuluslocation) (`bSuccessfullySensed` _bsuccessfullysensed)) (break `AIStimulus` (`local.Stimulus`)))
  (bind _returnvalue (`AIPerceptionSystem.GetSenseClassForStimulus` Stimulus))
  (if (== _returnvalue "/Script/AIModule.AISense_Hearing")
    (if _bsuccessfullysensed
      (`BlackboardComponent.SetValueAsVector` (`AIController.Blackboard` (`AIBlueprintHelperLibrary.GetAIController` self)) "LastKnownLocation" _stimuluslocation)
      (`BlackboardComponent.SetValueAsBool` (`AIController.Blackboard` (`AIBlueprintHelperLibrary.GetAIController` self)) "Investigating" true)
      (else
        (return)))
    (else
      (return))))

(fn `HandleSight`
  (params (SensedActor :type "Actor Object Reference") (Stimulus :type "AIStimulus Structure"))
  (bind ((`StimulusLocation` _stimuluslocation) (`bSuccessfullySensed` _bsuccessfullysensed)) (break `AIStimulus` (`local.Stimulus`)))
  (bind _returnvalue (`AIPerceptionSystem.GetSenseClassForStimulus` Stimulus))
  (if (== _returnvalue "/Script/AIModule.AISense_Sight")
    (if (== (`local.SensedActor`) (`GameplayStatics.GetPlayerCharacter` 0))
      (`BlackboardComponent.SetValueAsObject` (`AIController.Blackboard` (`AIBlueprintHelperLibrary.GetAIController` self)) "TargetActor" (select `bool` _bsuccessfullysensed :`true` (`local.SensedActor`) :!type "Object Object Reference"))
      (if (not _bsuccessfullysensed)
        (`BlackboardComponent.SetValueAsVector` (`AIController.Blackboard` (`AIBlueprintHelperLibrary.GetAIController` self)) "LastKnownLocation" _stimuluslocation))
      (else
        (return)))
    (else
      (return))))

(fn `UserConstructionScript`)