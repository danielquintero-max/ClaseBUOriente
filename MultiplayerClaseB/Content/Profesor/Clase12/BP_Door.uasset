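; Interactive door Blueprint that toggles open and closed each time it receives an Interacted event.
; A timeline plays forward or in reverse, lerping the mesh's yaw between closed and a quarter-turn open.
; When the timeline finishes, it sets a referenced nav modifier to the default area if open or null if closed, so AI navigation follows the door state.
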(event `Interacted`
  (bind _output_get (set `self.DoorOpen` (not (`self.DoorOpen`))))
  (if _output_get
    (`self.OpenDoor`)
    (else
      (`self.CloseDoor`))))

(event `OpenDoor`
  (bind _navmodifierreference (`self.NavModifierReference`))
  (bind (_direction _doorrotationtrack) (`Timeline|Timeline` :!label _label)
    (:`Update`
      (`SceneComponent.K2_SetRelativeRotation` (`self.StaticMesh1`) (`KismetMathLibrary.MakeRotator` 0.0 0.0 (`KismetMathLibrary.Lerp` 0.0 -90.0 _doorrotationtrack)) false false))
    (:`Finished`
      (switch `ETimelineDirection` _direction
        (:`Forward`
          (`/Engine/EditorBlueprintResources/StandardMacros.IsValid` _navmodifierreference
            (:`Is Valid`
              (`NavModifierVolume.SetAreaClass` _navmodifierreference "/Script/NavigationSystem.NavArea_Default"))))
        (:`Backward`
          (`/Engine/EditorBlueprintResources/StandardMacros.IsValid` _navmodifierreference
            (:`Is Valid`
              (`NavModifierVolume.SetAreaClass` _navmodifierreference "/Script/NavigationSystem.NavArea_Null"))))))))

(event `CloseDoor`
  (goto _label :!via `Reverse`))

(fn `UserConstructionScript`)